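; Base avatar Blueprint that lets a living avatar collect pickup items by walking into them.
; Actor overlap calls TryPickUpItem, which checks the health component, casts the other actor to PickupItem and offers its Id to the PickupManager.
; On success the item is taken, and destroyed only if it has no valid owner, since owners such as spawn points manage their pickups' lifetime.
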(event `self.ReceiveActorBeginOverlap`
  (params (OtherActor :type "Actor Object Reference"))
  (`self.TryPickUpItem` OtherActor))

(fn `TryPickUpItem`
  (params (otherActor :type "Actor Object Reference"))
  (if (`HealthComponent.IsAlive` (`self.BP_HealthComponent`))
    (`/Engine/EditorBlueprintResources/StandardMacros.IsValid` otherActor
      (:`Is Valid`
        (bind _aspickup_item (cast `PickupItem` otherActor))
        (bind _returnvalue (`PickupManagerComponent.TryPickUpItem` (`self.PickupManager`) (`PickupItem._id` _aspickup_item)))
        (if _returnvalue
          (`PickupItem.Take` _aspickup_item)
          ;[1 1 1] Pickup owner (e.g. pickup spawn point) handles it's life time. No owner - pickup life time is handled here
          (`/Engine/EditorBlueprintResources/StandardMacros.IsValid` (`self.GetOwner` _aspickup_item)
            (:`Is Not Valid`
              (`self.K2_DestroyActor` _aspickup_item))))))))

(fn `UserConstructionScript`)