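; Player avatar sound component that plays footstep, jump and landing effects as non-positional 2D audio.
; Step, jump and land events each trigger playback, with jump and land using one fixed sound apiece.
; Footsteps cycle in order through the StepSounds array via a wrapping index, with the array length cached at BeginPlay.
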(event `self.ReceiveBeginPlay`
  ;[1 1 1] Initialization
  (set `self.MaxStepSoundIndex` (`KismetArrayLibrary.Array_Length` (`self.StepSounds`))))

(event `self.BpOnStep`
  ;[1 1 1] On Step
  (bind _stepsound (`self.GetStepSound`))
  (`GameplayStatics.PlaySound2D` _stepsound 1.0 1.0 0.0 null null false))

(event `self.BpOnJump`
  ;[1 1 1] On Jump
  (`GameplayStatics.PlaySound2D` "/Game/Assets/SoundEffects/Q3/Steps/Sfx_q3_jump1.Sfx_q3_jump1" 1.0 1.0 0.0 null null false))

(event `self.BpOnLand`
  ;[1 1 1] On Land
  (`GameplayStatics.PlaySound2D` "/Game/Assets/SoundEffects/Q3/Steps/Sfx_q3_land1.Sfx_q3_land1" 1.0 1.0 0.0 null null false))

(fn `GetStepSound`
  (returns (StepSound :type "SoundBase Object Reference"))
  (bind _returnvalue (+ (`self.StepSoundIndex`) 1))
  (if (> (`self.MaxStepSoundIndex`) 0)
    (set `self.StepSoundIndex` _returnvalue)
    (if (> _returnvalue (`self.MaxStepSoundIndex`))
      (set `self.StepSoundIndex` 0))
    (return (`|GetArrayItem` (`self.StepSounds`) (`self.StepSoundIndex`)))
    (else
      (return null))))