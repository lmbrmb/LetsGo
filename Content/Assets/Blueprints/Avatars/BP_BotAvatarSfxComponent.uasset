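; Bot avatar sound component that plays footstep, jump and landing effects at the owning actor's location.
; Step, jump and land events each play a one-shot sound using the shared avatar attenuation settings.
; Footsteps cycle sequentially through the StepSounds array, whose length is cached at BeginPlay, while jump and land use fixed sounds.
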(event `self.ReceiveBeginPlay`
  ;[1 1 1] Initialization
  (set `self.MaxStepSoundIndex` (`KismetArrayLibrary.Array_Length` (`self.StepSounds`))))

(event `self.BpOnStep`
  ;[1 1 1] On Step
  (bind _stepsound (`self.GetStepSound`))
  (`GameplayStatics.PlaySoundAtLocation` _stepsound (`Actor.K2_GetActorLocation` (`self.GetOwner`)) (struct) 1.0 1.0 0.0 "/Game/Assets/Blueprints/SoundAttenuation/SA_Avatar.SA_Avatar" null null))

(event `self.BpOnJump`
  ;[1 1 1] On Jump
  (`GameplayStatics.PlaySoundAtLocation` "/Game/Assets/SoundEffects/Q3/Steps/Sfx_q3_jump1.Sfx_q3_jump1" (`Actor.K2_GetActorLocation` (`self.GetOwner`)) (struct) 1.0 1.0 0.0 "/Game/Assets/Blueprints/SoundAttenuation/SA_Avatar.SA_Avatar" null null))

(event `self.BpOnLand`
  ;[1 1 1] On Land
  (`GameplayStatics.PlaySoundAtLocation` "/Game/Assets/SoundEffects/Q3/Steps/Sfx_q3_land1.Sfx_q3_land1" (`Actor.K2_GetActorLocation` (`self.GetOwner`)) (struct) 1.0 1.0 0.0 "/Game/Assets/Blueprints/SoundAttenuation/SA_Avatar.SA_Avatar" null null))

(fn `GetStepSound`
  (returns (StepSound :type "SoundBase Object Reference"))
  (bind _returnvalue (+ (`self.StepSoundIndex`) 1))
  (if (> (`self.MaxStepSoundIndex`) 0)
    (set `self.StepSoundIndex` _returnvalue)
    (if (> _returnvalue (`self.MaxStepSoundIndex`))
      (set `self.StepSoundIndex` 0))
    (return (`|GetArrayItem` (`self.StepSounds`) (`self.StepSoundIndex`)))
    (else
      (return null))))