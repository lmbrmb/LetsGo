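; Player avatar SFX component that plays footstep, jump and landing sounds for the player's character.
; Setter events store the jump and land sounds and append step sounds to an array.
; Step, jump and land events play them as non-UI 2D sounds, with GetStepSound cycling through the step array in order and wrapping to the start.
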(event `self.BpSetJumpSound`
  (params (jumpSound :type "SoundBase Object Reference"))
  ;[1 1 1] Initialization
  (set `self.JumpSound` jumpSound))

(event `self.BpSetLandSound`
  (params (jumpSound :type "SoundBase Object Reference"))
  ;[1 1 1] Initialization
  (set `self.LandSound` jumpSound))

(event `self.BpAddStepSound`
  (params (jumpSound :type "SoundBase Object Reference"))
  ;[1 1 1] Initialization
  (`KismetArrayLibrary.Array_Add` (`self.StepSounds`) jumpSound))

(event `self.BpOnStep`
  ;[1 1 1] On Step
  (bind _stepsound (`self.GetStepSound`))
  (`GameplayStatics.PlaySound2D` _stepsound 1.0 1.0 0.0 null null false))

(event `self.BpOnJump`
  ;[1 1 1] On Jump
  (`GameplayStatics.PlaySound2D` (`self.JumpSound`) 1.0 1.0 0.0 null null false))

(event `self.BpOnLand`
  ;[1 1 1] On Land
  (`GameplayStatics.PlaySound2D` (`self.LandSound`) 1.0 1.0 0.0 null null false))

(fn `GetStepSound`
  (returns (StepSound :type "SoundBase Object Reference"))
  (bind _returnvalue (`KismetArrayLibrary.Array_Length` (`self.StepSounds`)))
  (bind _returnvalue_2 (+ (`self.StepSoundIndex`) 1))
  (if (> _returnvalue 0)
    (set `self.StepSoundIndex` _returnvalue_2)
    (if (> _returnvalue_2 _returnvalue)
      (set `self.StepSoundIndex` 0))
    (return (`|GetArrayItem` (`self.StepSounds`) (`self.StepSoundIndex`)))
    (else
      (return null))))