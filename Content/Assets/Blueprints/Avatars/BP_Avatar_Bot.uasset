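; BP_Avatar_Bot is the avatar Blueprint for bots, handling weapon setup and item pickup.
; On BeginPlay it passes its skeletal mesh to the bot weapon manager as the owner mesh.
; When it overlaps a PickupItem, it offers the item's Id to the PickupManager and calls Take on the item only if the pickup succeeds.
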(event `self.ReceiveBeginPlay`
  ;[1 1 1] Initialize weapon manager
  (`WeaponManagerComponent.SetOwnerSkeletalMeshComponent` (`self.BP_WeaponManager_Bot`) (`self.SkeletalMesh`)))

(event `self.ReceiveActorBeginOverlap`
  (params (OtherActor :type "Actor Object Reference"))
  ;[1 1 1] Pickup item
  (`/Engine/EditorBlueprintResources/StandardMacros.IsValid` OtherActor
    (:`Is Valid`
      (bind _aspickup_item (cast `PickupItem` OtherActor))
      (bind _returnvalue (`PickupManagerComponent.TryPickUpItem` (`self.PickupManager`) (`PickupItem._id` _aspickup_item)))
      (if _returnvalue
        (`PickupItem.Take` _aspickup_item)))))

(fn `UserConstructionScript`)