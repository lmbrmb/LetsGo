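; Machinegun Blueprint that supplies the fire pivot and the sound and visual feedback for gun events.
; Each shot plays the next sound in a cycled list and spawns a pooled Niagara muzzle flare at the firing pivot.
; Blocking bullet hits spawn pooled sparks along the impact normal, plus a random ricochet sound when no damage is dealt.
; Shot audio gets distance attenuation only when the owner is not the first player's pawn.
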(event `self.ReceiveBeginPlay`
  ;[1 1 1] Set FirePivots
  (`KismetArrayLibrary.Array_Add` (`self._firePivots`) (`self.FirePivot`))
  ;[1 1 1] Set ShotSoundsCount
  (set `self.ShotSoundsCount` (`KismetArrayLibrary.Array_Length` (`self.ShotSounds`)))
  ;[1 1 1] Set shot sound attenuation
  (if (not (== (`GameplayStatics.GetPlayerPawn` 0) (`self.GetOwner`)))
    (set `AudioComponent.AttenuationSettings` "/Game/Assets/Blueprints/SoundAttenuation/SA_GunShot.SA_GunShot" (`self.ShotAudioComponent`))))

(event `self.BpOnFireStarted`
  ;[1 1 1] OnFireStarted
  (set `self.IsFireStarted` true))

(event `self.BpOnFireStopped`
  ;[1 1 1] OnFireStopped
  (set `self.IsFireStarted` false))

(event `self.BpOnShotPerformed`
  (params (firePivot :type "SceneComponent Object Reference") (isAnyBulletDamaged :type Boolean))
  (bind _shotaudiocomponent (`self.ShotAudioComponent`))
  ;[1 1 1] SFX: set / play shot sound
  (bind _firesound (`self.CycleShotSound`))
  (`AudioComponent.SetSound` _shotaudiocomponent _firesound)
  (`AudioComponent.Play` _shotaudiocomponent 0.0)
  (`NiagaraFunctionLibrary.SpawnSystemAttached` "/Game/Assets/ParticleEffects/Flares/Machinegun/NiagaraSystem_MachinegunFlare.NiagaraSystem_MachinegunFlare" firePivot "None" (0.0 0.0 0.0) (struct) "KeepRelativeOffset" true true "AutoRelease") ; VFX: flare
)

(event `self.BpOnBulletTraced`
  (params (isDamaged :type Boolean) (hitResult :type "HitResult Structure (by ref)"))
  (bind (_bblockinghit _binitialoverlap _time _distance _location _impactpoint _normal _impactnormal) (`GameplayStatics.BreakHitResult` hitResult))
  ;[1 1 1] VFX: hit particles
  (if _bblockinghit
    (`NiagaraFunctionLibrary.SpawnSystemAtLocation` "/Game/Assets/ParticleEffects/NiagaraSystem_HitSparks.NiagaraSystem_HitSparks" _impactpoint (`KismetMathLibrary.MakeRotFromX` _impactnormal) (1.0 1.0 1.0) true true "AutoRelease")
    ;[1 1 1] SFX: Ricochet sound
    (if (not isDamaged)
      (`GameplayStatics.PlaySoundAtLocation` (`KismetArrayLibrary.Array_Random` (`self.RicochetSounds`)) _impactpoint (struct) 1.0 1.0 0.0 "/Game/Assets/Blueprints/SoundAttenuation/SA_GunShot.SA_GunShot" null null))))

(fn `CycleShotSound`
  (returns (fireSound :type "SoundBase Object Reference"))
  (bind _output_get (set `self.ShotSoundIndex` (+ (`self.ShotSoundIndex`) 1)))
  (if (>= _output_get (`self.ShotSoundsCount`))
    (set `self.ShotSoundIndex` 0))
  (return (`|GetArrayItem` (`self.ShotSounds`) (`self.ShotSoundIndex`))))

(fn `UserConstructionScript`)