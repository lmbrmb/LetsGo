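; BP_ShotgunQ3 is a shotgun Blueprint that supplies the visual and audio feedback for shots, using a Quake 3 shot sound.
; BeginPlay sets the fire pivot, registers two barrel pivots and configures audio as non-spatial when the owner is player pawn 0, attenuated otherwise.
; Shot requests spawn a muzzle flare, per-barrel buckshot bursts with a set cone angle, and play the sound.
; Bullet traces spawn sparks on non-damaging blocking hits.
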(event `self.ReceiveBeginPlay`
  (bind _barrelpivots (`self.BarrelPivots`))
  ;[1 1 1] Set FirePivot
  (`self.SetFirePivot` (`self.FirePivot`))
  (`self.InitializeAudioComponent`)
  ;[1 1 1] Set shot sound
  (`AudioComponent.SetSound` (`self.AudioComponent`) "/Game/Assets/SoundEffects/Q3/Shotgun/Sfx_q3_sshotf1b.Sfx_q3_sshotf1b")
  ;[1 1 1] Populate barrel pivots
  (`KismetArrayLibrary.Array_Add` _barrelpivots (`self.BarrelPivot1`))
  (`KismetArrayLibrary.Array_Add` _barrelpivots (`self.BarrelPivot2`)))

(event `self.BpOnShotRequest`
  (params (firePivot :type "SceneComponent Object Reference"))
  (`NiagaraFunctionLibrary.SpawnSystemAttached` "/Game/Assets/ParticleEffects/Flares/Shotgun/NiagaraSystem_ShotgunFlare.NiagaraSystem_ShotgunFlare" firePivot "None" (0.0 0.0 0.0) (struct) "KeepRelativeOffset" true true "AutoRelease") ; VFX: Flare
  (`self.SpawnBuckshotVfx`)
  ;[1 1 1] SFX: play shot sound
  (`AudioComponent.Play` (`self.AudioComponent`) 0.0))

(event `self.BpOnBulletTraced`
  (params (isDamaged :type Boolean) (hitResult :type "HitResult Structure (by ref)"))
  (`self.SpawnHitVfx` isDamaged hitResult))

(fn `InitializeAudioComponent`
  (bind _audiocomponent (`self.AudioComponent`))
  (if (== (`GameplayStatics.GetPlayerPawn` 0) (`self.GetOwner`))
    (set `AudioComponent.AttenuationSettings` null _audiocomponent)
    (set `AudioComponent.bAllowSpatialization` false _audiocomponent)
    (else
      (set `AudioComponent.AttenuationSettings` "/Game/Assets/Blueprints/SoundAttenuation/SA_GunShot.SA_GunShot" _audiocomponent)
      (set `AudioComponent.bAllowSpatialization` true _audiocomponent))))

(fn `SpawnBuckshotVfx`
  (for _array_element (`self.BarrelPivots`)
    (bind _returnvalue (`NiagaraFunctionLibrary.SpawnSystemAtLocation` "/Game/Assets/ParticleEffects/NiagaraSystem_ShotgunBurst.NiagaraSystem_ShotgunBurst" (`SceneComponent.K2_GetComponentLocation` _array_element) (`SceneComponent.K2_GetComponentRotation` _array_element) (1.0 1.0 1.0) true true "AutoRelease"))
    (`NiagaraComponent.SetVariableFloat` _returnvalue (`self.NiagaraConeAngleName`) (`self.NiagaraConeAngleValue`))))

(fn `SpawnHitVfx`
  (params (isDamaged :type Boolean) (hitResult :type "HitResult Structure"))
  (bind (_bblockinghit _binitialoverlap _time _distance _location _impactpoint _normal _impactnormal) (`GameplayStatics.BreakHitResult` hitResult))
  (if (and (not isDamaged) _bblockinghit)
    (`NiagaraFunctionLibrary.SpawnSystemAtLocation` "/Game/Assets/ParticleEffects/NiagaraSystem_HitSparks.NiagaraSystem_HitSparks" _impactpoint (`KismetMathLibrary.MakeRotFromX` _impactnormal) (1.0 1.0 1.0) true true "AutoRelease")))

(fn `UserConstructionScript`)