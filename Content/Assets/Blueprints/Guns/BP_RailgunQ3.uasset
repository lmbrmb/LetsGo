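; Quake 3-style railgun Blueprint that adds firing sound and a beam effect to the gun's shot and trace events.
; On BeginPlay it sets the fire pivot and shot sound, playing unspatialized when the owner is the first player's pawn and attenuated otherwise.
; Each bullet trace spawns a pooled Niagara beam to the impact or trace end.
; Beam sparkle box and particle count scale with ray length.
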(event `self.ReceiveBeginPlay`
  ;[1 1 1] Set FirePivot
  (`self.SetFirePivot` (`self.FirePivot`))
  (`self.InitializeAudioComponent`)
  ;[1 1 1] Set shot sound
  (`AudioComponent.SetSound` (`self.AudioComponent`) "/Game/Assets/SoundEffects/Q3/Railgun/Sfx_q3_railgf1a.Sfx_q3_railgf1a") ; Set shot sound
)

(event `self.BpOnBulletTraced`
  (params (isDamaged :type Boolean) (hitResult :type "HitResult Structure (by ref)"))
  (`self.SpawnBeamVfx` hitResult))

(event `self.BpOnShotRequest`
  (params (firePivot :type "SceneComponent Object Reference"))
  ;[1 1 1] SFX: Play shot sound
  (`AudioComponent.Play` (`self.AudioComponent`) 0.0))

(fn `InitializeAudioComponent`
  (bind _audiocomponent (`self.AudioComponent`))
  (if (== (`GameplayStatics.GetPlayerPawn` 0) (`self.GetOwner`))
    (set `AudioComponent.AttenuationSettings` null _audiocomponent)
    (set `AudioComponent.bAllowSpatialization` false _audiocomponent)
    (else
      (set `AudioComponent.AttenuationSettings` "/Game/Assets/Blueprints/SoundAttenuation/SA_GunShot.SA_GunShot" _audiocomponent)
      (set `AudioComponent.bAllowSpatialization` true _audiocomponent))))

(fn `SpawnBeamVfx`
  (params (hitResult :type "HitResult Structure"))
  (bind (_bblockinghit _binitialoverlap _time _distance _location _impactpoint _normal _impactnormal _physmat _hitactor _hitcomponent _hitbonename _hititem _faceindex _tracestart _traceend) (`GameplayStatics.BreakHitResult` hitResult))
  (bind _returnvalue (`KismetMathLibrary.SelectVector` _impactpoint _traceend _bblockinghit))
  (bind _returnvalue_2 (- _returnvalue _tracestart))
  (bind _returnvalue_3 (`KismetMathLibrary.VSize` _returnvalue_2))
  (bind _returnvalue_4 (`NiagaraFunctionLibrary.SpawnSystemAtLocation` "/Game/Assets/ParticleEffects/NiagaraSystem_RailgunBeam.NiagaraSystem_RailgunBeam" _tracestart (`KismetMathLibrary.MakeRotFromX` _returnvalue_2) (1.0 1.0 1.0) true true "AutoRelease"))
  (`NiagaraComponent.SetVariableVec3` _returnvalue_4 (`self.NiagaraParamName_BeamEndLocation`) _returnvalue)
  (`NiagaraComponent.SetVariableLinearColor` _returnvalue_4 (`self.NiagaraParamName_BeamColor`) (`self.NiagaraBeamColorVector`))
  (`NiagaraComponent.SetVariableVec3` _returnvalue_4 (`self.NiagaraParamName_BeamSparklesBoxSize`) (`KismetMathLibrary.MakeVector` _returnvalue_3 1.0 1.0))
  (`NiagaraComponent.SetVariableVec3` _returnvalue_4 (`self.NiagaraParamName_BeamSparklesBoxOffset`) (`KismetMathLibrary.MakeVector` (/ _returnvalue_3 2.0) 1.0 1.0))
  (`NiagaraComponent.SetVariableInt` _returnvalue_4 (`self.NiagaraParamName_BeamSparklesCount`) (`KismetMathLibrary.FTrunc` (* (`self.BeamSparklesMax`) (/ _returnvalue_3 (`self.BeamSparklesBaseRayLength`))))))

(fn `UserConstructionScript`)