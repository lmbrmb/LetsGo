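; BP_Railgun is a railgun weapon Blueprint that supplies the firing visuals and sound for traced shots.
; It registers its fire pivot on BeginPlay and sets up the shot sound, applying gunshot attenuation only when its owner is not the player pawn.
; Each bullet trace spawns a Niagara beam from trace start to impact point, or to trace end on a miss.
; Each performed shot plays the sound.
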(event `self.ReceiveBeginPlay`
  (bind _shotaudiocomponent (`self.ShotAudioComponent`))
  ;[1 1 1] Initialization
  (`KismetArrayLibrary.Array_Add` (`self._firePivots`) (`self.FirePivot`))
  (`AudioComponent.SetSound` _shotaudiocomponent "/Game/Assets/SoundEffects/Sfx_RailgunShot1.Sfx_RailgunShot1") ; Set shot sound
  ;[1 1 1] Set shot sound attenuation
  (if (not (== (`GameplayStatics.GetPlayerPawn` 0) (`self.GetOwner`)))
    (set `AudioComponent.AttenuationSettings` "/Game/Assets/Blueprints/SoundAttenuation/SA_GunShot.SA_GunShot" _shotaudiocomponent)))

(event `self.BpOnBulletTraced`
  (params (isDamaged :type Boolean) (hitResult :type "HitResult Structure (by ref)"))
  (bind (_bblockinghit _binitialoverlap _time _distance _location _impactpoint _normal _impactnormal _physmat _hitactor _hitcomponent _hitbonename _hititem _faceindex _tracestart _traceend) (`GameplayStatics.BreakHitResult` hitResult))
  ;[1 1 1] VFX: Beam
  (bind _returnvalue (`NiagaraFunctionLibrary.SpawnSystemAtLocation` "/Game/Assets/ParticleEffects/NiagaraSystem_RailgunBeam.NiagaraSystem_RailgunBeam" _tracestart))
  (`NiagaraComponent.SetVariableVec3` _returnvalue (`self.NiagaraBeamEndLocationName`) (`KismetMathLibrary.SelectVector` _impactpoint _traceend _bblockinghit)))

(event `self.BpOnShotPerformed`
  (params (firePivot :type "SceneComponent Object Reference") (isAnyBulletDamaged :type Boolean))
  ;[1 1 1] SFX: Play shot sound
  (`AudioComponent.Play` (`self.ShotAudioComponent`) 0.0))

(fn `UserConstructionScript`)