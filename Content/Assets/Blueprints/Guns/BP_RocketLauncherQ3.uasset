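; BP_RocketLauncherQ3 is a rocket launcher weapon Blueprint, named after the Quake 3 weapon.
; On BeginPlay it fills its FirePivots array, starting with FirePivot1, and assigns a Quake 3 shot sound to its audio component.
; When the owner is not the first player's pawn, it applies gunshot attenuation settings to that audio component.
; The graph holds only this setup, with no firing logic of its own.
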(event `self.ReceiveBeginPlay`
  (bind _shotaudiocomponent (`self.ShotAudioComponent`))
  (bind __firepivots (`self._firePivots`))
  ;[1 1 1] Initialization
  (`KismetArrayLibrary.Array_Add` __firepivots (`self.FirePivot1`))
  (`KismetArrayLibrary.Array_Add` __firepivots)
  (`AudioComponent.SetSound` _shotaudiocomponent "/Game/Assets/SoundEffects/Q3/Sfx_q3_sshotf1b.Sfx_q3_sshotf1b") ; Set shot sound
  ;[1 1 1] Set shot sound attenuation
  (if (not (== (`GameplayStatics.GetPlayerPawn` 0) (`self.GetOwner`)))
    (set `AudioComponent.AttenuationSettings` "/Game/Assets/Blueprints/SoundAttenuation/SA_GunShot.SA_GunShot" _shotaudiocomponent)))

(fn `UserConstructionScript`)