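; Minigun weapon Blueprint that supplies the fire pivot and the sound and VFX responses to firing events.
; BeginPlay registers the pivot and applies gunshot attenuation to shot audio unless the owner is the player pawn.
; Fire start and stop set the fire flag and switch gun audio between loop and stop sounds.
; Shots spawn an attached muzzle flare; blocking hits spawn pooled sparks, plus a random ricochet sound when no damage is dealt.
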(event `self.ReceiveBeginPlay`
  ;[1 1 1] Set FirePivots
  (`KismetArrayLibrary.Array_Add` (`self._firePivots`) (`self.FirePivot`))
  ;[1 1 1] Set shot sound attenuation
  (if (not (== (`GameplayStatics.GetPlayerPawn` 0) (`self.GetOwner`)))
    (set `AudioComponent.AttenuationSettings` "/Game/Assets/Blueprints/SoundAttenuation/SA_GunShot.SA_GunShot" (`self.ShotAudioComponent`))))

(event `self.BpOnFireStarted`
  (bind _gunaudiocomponent (`self.GunAudioComponent`))
  ;[1 1 1] OnFireStarted
  (set `self.IsFireStarted` true)
  ;[1 1 1] SFX: Fire loop
  (`AudioComponent.SetSound` _gunaudiocomponent (`self.MinigunLoopSound`))
  (`AudioComponent.Play` _gunaudiocomponent 0.0))

(event `self.BpOnFireStopped`
  (bind _gunaudiocomponent (`self.GunAudioComponent`))
  ;[1 1 1] OnFireStopped
  (set `self.IsFireStarted` false)
  (`AudioComponent.SetSound` _gunaudiocomponent (`self.MinigunStopSound`))
  (`AudioComponent.Play` _gunaudiocomponent 0.0))

(event `self.BpOnBulletTraced`
  (params (isDamaged :type Boolean) (hitResult :type "HitResult Structure (by ref)"))
  (bind (_bblockinghit _binitialoverlap _time _distance _location _impactpoint _normal _impactnormal) (`GameplayStatics.BreakHitResult` hitResult))
  ;[1 1 1] VFX: hit particles
  (if _bblockinghit
    (`NiagaraFunctionLibrary.SpawnSystemAtLocation` "/Game/Assets/ParticleEffects/NiagaraSystem_HitSparks.NiagaraSystem_HitSparks" _impactpoint (`KismetMathLibrary.MakeRotFromX` _impactnormal) (1.0 1.0 1.0) true true "AutoRelease")
    ;[1 1 1] SFX: Ricochet sound
    (if (not isDamaged)
      (`GameplayStatics.PlaySoundAtLocation` (`KismetArrayLibrary.Array_Random` (`self.RicochetSounds`)) _impactpoint (struct) 1.0 1.0 0.0 "/Game/Assets/Blueprints/SoundAttenuation/SA_GunShot.SA_GunShot" null null))))

(event `self.BpOnShotPerformed`
  (params (firePivot :type "SceneComponent Object Reference") (isAnyBulletDamaged :type Boolean))
  (`NiagaraFunctionLibrary.SpawnSystemAttached` "/Game/Assets/ParticleEffects/Flares/Machinegun/NiagaraSystem_MachinegunFlare.NiagaraSystem_MachinegunFlare" firePivot "None" (0.0 0.0 0.0) (struct) "KeepRelativeOffset" true true "AutoRelease") ; VFX: flare
)

(fn `UserConstructionScript`)