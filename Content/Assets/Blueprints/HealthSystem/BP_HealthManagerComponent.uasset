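; Health manager component Blueprint that handles the visual and loot reactions when its owner is hit, dies or is overkilled.
; Blocking hits spawn an attached, pooled Niagara blood spurt at the impact point.
; Death uses a downward trace to place a pickup of the owner's current weapon ID through its PickupSpawnComponent.
; Overkill spawns a random gibs effect and hides all of the owner's skeletal meshes.
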(event `self.BpOnDied`
  (`self.SpawnPickup`))

(event `self.BpOnHit`
  (params (hitResult :type "HitResult Structure (by ref)"))
  (`self.SpawnHitVfx` hitResult))

(event `self.BpOnOverkill`
  (`self.SpawnGibsVfx`)
  (`self.MakeInvisible`))

(fn `MakeInvisible`
  (for _array_element (`Actor.K2_GetComponentsByClass` (`self.GetOwner`) "/Script/Engine.SkeletalMeshComponent")
    (`SceneComponent.SetVisibility` _array_element false true)))

(fn `SpawnGibsVfx`
  (`NiagaraFunctionLibrary.SpawnSystemAtLocation` (`KismetArrayLibrary.Array_Random` (`self.GibsNiagaraSystems`)) (+ (`SceneComponent.K2_GetComponentLocation` (`Actor.RootComponent` (`self.GetOwner`))) (0.0 0.0 100.0)) (struct) (1.0 1.0 1.0) true true "AutoRelease"))

(fn `SpawnHitVfx`
  (params (hitResult :type "HitResult Structure"))
  (bind (_bblockinghit _binitialoverlap _time _distance _location _impactpoint) (`GameplayStatics.BreakHitResult` hitResult))
  (if _bblockinghit
    (`NiagaraFunctionLibrary.SpawnSystemAttached` "/Game/Assets/ParticleEffects/BloodSpurt/NiagaraSystem_BloodSpurt.NiagaraSystem_BloodSpurt" (`Actor.RootComponent` (`self.GetOwner`)) "None" _impactpoint (`KismetMathLibrary.MakeRotFromX` _impactpoint) "KeepWorldPosition" true true "AutoRelease")
    (else
      (`KismetSystemLibrary.PrintString` "Not blocking hit"))))

(fn `SpawnPickup`
  (bind _returnvalue (`self.GetOwner`))
  (bind _returnvalue_2 (`Actor.GetComponentByClass` _returnvalue "/Script/LetsGo.PickupSpawnComponent"))
  (bind _returnvalue_3 (`Actor.GetComponentByClass` _returnvalue "/Script/LetsGo.WeaponManagerComponent"))
  (bind _returnvalue_4 (`WeaponManagerComponent.GetCurrentWeaponId` _returnvalue_3))
  (bind _returnvalue_5 (`SceneComponent.K2_GetComponentLocation` (`Actor.RootComponent` _returnvalue)))
  (`/Engine/EditorBlueprintResources/StandardMacros.IsValid` _returnvalue_3
    (:`Is Valid`
      (switch `name` _returnvalue_4
        (:`Default`
          (`/Engine/EditorBlueprintResources/StandardMacros.IsValid` _returnvalue_2
            (:`Is Valid`
              (bind _outhit (`KismetSystemLibrary.LineTraceSingle` _returnvalue_5 (+ _returnvalue_5 (0.0 0.0 -1000.0)) "TraceTypeQuery1"))
              (bind (_bblockinghit _binitialoverlap _time _distance _location _impactpoint) (`GameplayStatics.BreakHitResult` _outhit))
              (`PickupSpawnComponent.SpawnPickup` _returnvalue_2 _returnvalue_4 (+ (`KismetMathLibrary.SelectVector` _impactpoint _location _bblockinghit) (0.0 0.0 100.0))))))))))