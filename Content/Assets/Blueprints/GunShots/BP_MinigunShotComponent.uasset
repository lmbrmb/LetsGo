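; Minigun shot component that supplies the weapon's firing and ricochet audio.
; Each shot steps through the fire sound array in order, playing it in 2D for the local player or at the fire pivot for others.
; Local status is cached at BeginPlay by comparing player pawn 0 to the owner's owner.
; Bullets with a blocking hit but no damage play a random ricochet sound at the impact point.
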(event `self.ReceiveBeginPlay`
  ;[1 1 1] Set FireSoundsCount
  (set `self.FireSoundsCount` (`KismetArrayLibrary.Array_Length` (`self.FireSounds`)))
  ;[1 1 1] Set IsLocalPlayer
  (set `self.IsLocalPlayer` (== (`GameplayStatics.GetPlayerPawn` 0) (`Actor.GetOwner` (`self.GetOwner`)))))

(event `self.BpOnShotPerformed`
  (params (firePivot :type "SceneComponent Object Reference"))
  ;[1 1 1] SFX: shot sound
  (bind _firesound (`self.CycleFireSound`))
  (if (`self.IsLocalPlayer`)
    (`GameplayStatics.PlaySound2D` _firesound 1.0 1.0 0.0 null null false)
    (else
      (`GameplayStatics.PlaySoundAtLocation` _firesound (`SceneComponent.K2_GetComponentLocation` firePivot) (struct) 1.0 1.0 0.0 null null null))))

(event `self.BpOnBullet`
  (params (isDamaged :type Boolean) (hitResult :type "HitResult Structure"))
  (bind (_bblockinghit _binitialoverlap _time _distance _location) (`GameplayStatics.BreakHitResult` hitResult))
  ;[1 1 1] SFX: ricochet sound at impact location
  (if (and (not isDamaged) _bblockinghit)
    (`GameplayStatics.PlaySoundAtLocation` (`KismetArrayLibrary.Array_Random` (`self.RicochetSounds`)) _location (struct) 1.0 1.0 0.0 "/Game/Assets/Blueprints/SoundAttenuation/SA_GunShot.SA_GunShot" null null)))

(fn `CycleFireSound`
  (returns (fireSound :type "SoundBase Object Reference"))
  (bind _output_get (set `self.FireSoundIndex` (+ (`self.FireSoundIndex`) 1)))
  (if (>= _output_get (`self.FireSoundsCount`))
    (set `self.FireSoundIndex` 0))
  (return (`|GetArrayItem` (`self.FireSounds`) (`self.FireSoundIndex`))))