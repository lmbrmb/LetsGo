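; BP_RailgunShotComponent is the shot effects component for the railgun, handling the sound and beam visuals of each shot.
; On init it assigns the railgun shot sound and applies gunshot attenuation only for non-local players.
; Each shot plays the sound, and each bullet spawns a Niagara beam from the trace start to the impact point, or to the trace end when nothing is hit.
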(event `self.BpInit`
  (bind __audiocomponent (`self._audioComponent`))
  (`AudioComponent.SetSound` __audiocomponent "/Game/Assets/SoundEffects/Sfx_RailgunShot1.Sfx_RailgunShot1")
  ;[1 1 1] Set shot sound attenuation
  (if (not (`self.GetIsLocalPlayer`))
    (set `AudioComponent.AttenuationSettings` "/Game/Assets/Blueprints/SoundAttenuation/SA_GunShot.SA_GunShot" __audiocomponent)))

(event `self.BpOnBullet`
  (params (isDamaged :type Boolean) (hitResult :type "HitResult Structure"))
  (bind (_bblockinghit _binitialoverlap _time _distance _location _impactpoint _normal _impactnormal _physmat _hitactor _hitcomponent _hitbonename _hititem _faceindex _tracestart _traceend) (`GameplayStatics.BreakHitResult` hitResult))
  ;[1 1 1] VFX: Beam
  (bind _returnvalue (`NiagaraFunctionLibrary.SpawnSystemAtLocation` "/Game/Assets/ParticleEffects/NiagaraSystem_RailgunBeam.NiagaraSystem_RailgunBeam" _tracestart))
  (`NiagaraComponent.SetVariableVec3` _returnvalue (`self.NiagaraBeamEndLocationName`) (`KismetMathLibrary.SelectVector` _impactpoint _traceend _bblockinghit)))

(event `self.BpOnShotPerformed`
  (params (firePivot :type "SceneComponent Object Reference"))
  ;[1 1 1] SFX: Play shot sound
  (`AudioComponent.Play` (`self._audioComponent`) 0.0))