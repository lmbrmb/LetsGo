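; Movement component Blueprint for a bot avatar that plays footstep and landing sounds at the owning actor's location.
; Each step event takes the next entry from the StepSounds array through GetStepSound, which cycles an index and wraps at the length cached on BeginPlay.
; The land event plays its sound separately, outside that cycle.
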(event `self.ReceiveBeginPlay`
  (set `self.MaxStepSoundIndex` (`KismetArrayLibrary.Array_Length` (`self.StepSounds`))))

(event `self.BpOnStep`
  (bind _stepsound (`self.GetStepSound`))
  (`GameplayStatics.PlaySoundAtLocation` _stepsound (`Actor.K2_GetActorLocation` (`self.GetOwner`)) (struct) 1.0 1.0 0.0 null null null))

(event `self.BpOnLand`
  (`GameplayStatics.PlaySoundAtLocation` null (`Actor.K2_GetActorLocation` (`self.GetOwner`)) (struct) 1.0 1.0 0.0 null null null))

(fn `GetStepSound`
  (returns (StepSound :type "SoundBase Object Reference"))
  (bind _returnvalue (+ (`self.StepSoundIndex`) 1))
  (set `self.StepSoundIndex` _returnvalue)
  (if (> _returnvalue (`self.MaxStepSoundIndex`))
    (set `self.StepSoundIndex` 0))
  (return (`|GetArrayItem` (`self.StepSounds`) (`self.StepSoundIndex`))))