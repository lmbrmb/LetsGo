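; Sawed-off shotgun weapon Blueprint that supplies two fire pivots and reload audio.
; On BeginPlay it adds its two pivot references to the FirePivots array.
; Reload event hooks play sounds at the weapon's location: a click when reloading starts and finishes, and a shell-loading sound when ammo is loaded.
; It contains no firing or ammo logic of its own.
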(event `self.ReceiveBeginPlay`
  (bind __firepivots (`self._firePivots`))
  ;[1 1 1] Initialization
  (`KismetArrayLibrary.Array_Add` __firepivots (`self.FirePivot1`))
  (`KismetArrayLibrary.Array_Add` __firepivots (`self.FirePivot2`)))

(event `self.BpReloadStarted`
  ;[1 1 1] Reload
  (`GameplayStatics.PlaySoundAtLocation` "/Game/Assets/SoundEffects/Sfx_ShotgunClick1.Sfx_ShotgunClick1" (`self.K2_GetActorLocation`) (struct) 1.0 1.0 0.0 null null null))

(event `self.BpAmmoLoaded`
  ;[1 1 1] Reload
  (`GameplayStatics.PlaySoundAtLocation` "/Game/Assets/SoundEffects/Sfx_ShotgunLoadOneShell1.Sfx_ShotgunLoadOneShell1" (`self.K2_GetActorLocation`) (struct) 1.0 1.0 0.0 null null null))

(event `self.BpReloadFinished`
  ;[1 1 1] Reload
  (`GameplayStatics.PlaySoundAtLocation` "/Game/Assets/SoundEffects/Sfx_ShotgunClick1.Sfx_ShotgunClick1" (`self.K2_GetActorLocation`) (struct) 1.0 1.0 0.0 null null null))

(fn `UserConstructionScript`)