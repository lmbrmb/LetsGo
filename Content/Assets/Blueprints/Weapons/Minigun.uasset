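; Minigun weapon Blueprint that registers its fire pivot on begin play and drives the gun's firing and reload sounds.
; Fire start plays a spin-up sound, waits its duration, then switches to a loop sound only if firing is still active.
; Fire stop clears the flag and plays a wind-down sound on the same audio component, while reload plays a one-shot at the actor's location.
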(event `self.ReceiveBeginPlay`
  ;[1 1 1] Initialization
  (`KismetArrayLibrary.Array_Add` (`self._firePivots`) (`self.FirePivot`)))

(event `self.OnFireStarted`
  (bind _audiocomponent (`self.AudioComponent`))
  (bind _minigunstartsound (`self.MinigunStartSound`))
  ;[1 1 1] OnFireStarted
  (set `self.IsFireStarted` true)
  (`AudioComponent.SetSound` _audiocomponent _minigunstartsound)
  (`AudioComponent.Play` _audiocomponent 0.0)
  (`KismetSystemLibrary.Delay` (`SoundBase.Duration` _minigunstartsound))
  (if (`self.IsFireStarted`)
    (`AudioComponent.SetSound` _audiocomponent (`self.MinigunLoopSound`))
    (`AudioComponent.Play` _audiocomponent 0.0)))

(event `self.OnFireStopped`
  (bind _audiocomponent (`self.AudioComponent`))
  ;[1 1 1] OnFireStopped
  (set `self.IsFireStarted` false)
  (`AudioComponent.SetSound` _audiocomponent (`self.MinigunStopSound`))
  (`AudioComponent.Play` _audiocomponent 0.0))

(event `self.OnReloadStarted`
  ;[1 1 1] OnReload
  (`GameplayStatics.PlaySoundAtLocation` "/Game/Assets/SoundEffects/Reload1.Reload1" (`self.K2_GetActorLocation`) (struct) 1.0 1.0 0.0 null null null))

(fn `UserConstructionScript`)