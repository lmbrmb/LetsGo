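; BP_Minigun is a minigun weapon Blueprint that handles firing state and sound.
; On BeginPlay it registers its FirePivot in the FirePivots list.
; The fire started and stopped events toggle IsFireStarted and switch one AudioComponent between the looping fire sound and the stop sound.
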(event `self.ReceiveBeginPlay`
  ;[1 1 1] Initialization
  (`KismetArrayLibrary.Array_Add` (`self._firePivots`) (`self.FirePivot`)))

(event `self.BpFireStarted`
  (bind _audiocomponent (`self.AudioComponent`))
  ;[1 1 1] OnFireStarted
  (set `self.IsFireStarted` true)
  (`AudioComponent.SetSound` _audiocomponent (`self.MinigunLoopSound`))
  (`AudioComponent.Play` _audiocomponent 0.0))

(event `self.BpFireStopped`
  (bind _audiocomponent (`self.AudioComponent`))
  ;[1 1 1] OnFireStopped
  (set `self.IsFireStarted` false)
  (`AudioComponent.SetSound` _audiocomponent (`self.MinigunStopSound`))
  (`AudioComponent.Play` _audiocomponent 0.0))

(fn `UserConstructionScript`)