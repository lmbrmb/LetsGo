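; BP_Bot1 is a bot character that carries weapons and collects pickup items.
; On BeginPlay it registers its WeaponPivot with the WeaponManager as both aim provider and weapon pivot.
; When it overlaps a PickupItem, it tries to add the item's Id to its Inventory and destroys the pickup only if that succeeds.
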(event `self.ReceiveBeginPlay`
  (bind _weaponmanager (`self.WeaponManager`))
  (bind _weaponpivot (`self.WeaponPivot`))
  ;[1 1 1] Initialize weapon manager
  (`WeaponManagerComponent.SetAimProvider` _weaponmanager _weaponpivot)
  (`WeaponManagerComponent.AddWeaponPivot` _weaponmanager _weaponpivot))

(event `self.ReceiveActorBeginOverlap`
  (params (OtherActor :type "Actor Object Reference"))
  ;[1 1 1] OnActorBeginOverlap
  (`/Engine/EditorBlueprintResources/StandardMacros.IsValid` OtherActor
    (:`Is Valid`
      (bind _aspickup_item (cast `PickupItem` OtherActor))
      (bind _returnvalue (`InventoryComponent.TryAddItem` (`self.Inventory`) (`PickupItem._id` _aspickup_item)))
      (if _returnvalue
        (`self.K2_DestroyActor` OtherActor)))))

(fn `UserConstructionScript`)